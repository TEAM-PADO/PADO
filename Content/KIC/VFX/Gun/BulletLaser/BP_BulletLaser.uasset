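; BP_BulletLaser is a laser bullet effect actor that flies from its spawn point to a Destination and expires on arrival.
; On BeginPlay it faces Destination, sets its lifespan from distance at a fixed speed and moves its root over that time.
; It plays a gunshot sound and, if Hit is set, spawns BP_LaserSpark at Destination just before expiring.
; The construction script gives the Niagara beam a fixed length.
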(event `self.ReceiveBeginPlay`
  (bind _returnvalue (`self.K2_GetActorLocation`))
  (bind _destination (`self.Destination`))
  (bind _defaultsceneroot (`self.DefaultSceneRoot`))
  (bind _returnvalue_2 (/ (`KismetMathLibrary.Vector_Distance` _returnvalue _destination) 20000.0))
  (`self.K2_SetActorRotation` (`KismetMathLibrary.FindLookAtRotation` _returnvalue _destination) true)
  (`self.SetLifeSpan` _returnvalue_2)
  (`|ExecutionSequence`
    (:`then_0`
      (`KismetSystemLibrary.MoveComponentTo` _defaultsceneroot _destination (`SceneComponent.RelativeRotation` _defaultsceneroot) false false _returnvalue_2))
    (:`then_1`
      (`GameplayStatics.SpawnSoundAtLocation` "/Game/KIC/Sound/SE/GunFire/072807_heavy-machine-gun-50-caliber-39765.072807_heavy-machine-gun-50-caliber-39765" (`self.K2_GetActorLocation`) (struct) 1.0 1.0 0.0 null null)
      (if (`self.Hit`)
        (`KismetSystemLibrary.Delay` (- _returnvalue_2 0.01))
        (`|SpawnActorFromClass` "/Game/KIC/Trap/LaserTrap/BP_LaserSpark.BP_LaserSpark_C" (`KismetMathLibrary.MakeTransform` (`self.Destination`)) "Undefined" "MultiplyWithRoot" null null)))))

(fn `UserConstructionScript`
  (`FXSystemComponent.SetVectorParameter` (`self.Niagara`) "BeamEnd" (800.0 0.0 0.0)))