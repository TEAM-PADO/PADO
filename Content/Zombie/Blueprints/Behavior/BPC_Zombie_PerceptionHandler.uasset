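; Controller component for zombie AI that turns sight and hearing perception updates on pawns into target sensed, lost and forgotten events.
; Sighting a target also forces it on zombie AI controllers within the pawn's group perception radius.
; Losing sight reports lost, then starts a timer from the stimulus expiration age to report forgotten, cleared on re-sighting.
; Hearing reports sensed or forgotten directly; a similar damage handler exists but is not routed.
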(event `self.ReceiveBeginPlay`
  (bind _output_get (set `self.AiPerceptionComponent` (`Actor.GetComponentByClass` (`self.GetOwner`) "/Script/AIModule.AIPerceptionComponent")))
  (add `AIPerceptionComponent.OnTargetPerceptionUpdated` _output_get (`|CreateDelegate` :!event `OnTargetPerceptionUpdated_Event`))
  (bind _asbp_zombie_ai_controller_base (cast `/Game/Zombie/Blueprints/Behavior/BP_Zombie_AiController_Base` (`self.GetOwner`)))
  (bind _asbp_zombie_pawn (cast `/Game/Zombie/Blueprints/BP_Zombie_Pawn` (`Controller.K2_GetPawn` _asbp_zombie_ai_controller_base)))
  (set `self.Controlled BP_ZombiePawn` _asbp_zombie_pawn))

(fn `HandleDamagePerception`
  (params (Actor :type "Actor Object Reference") (Stimulus :type "AIStimulus Structure"))
  (bind _actor (`local.Actor`))
  (bind _stimulus (`local.Stimulus`))
  (if (`.bSuccessfullySensed` (break `AIStimulus` Stimulus))
    (`self.OnTargetSensed` _actor _stimulus)
    (else
      (`self.OnTargetForgotten` _actor _stimulus))))

(fn `HandleHearingPerception`
  (params (Actor :type "Actor Object Reference") (Stimulus :type "AIStimulus Structure"))
  (bind _actor (`local.Actor`))
  (bind _stimulus (`local.Stimulus`))
  (if (`.bSuccessfullySensed` (break `AIStimulus` Stimulus))
    (`self.OnTargetSensed` _actor _stimulus)
    (else
      (`self.OnTargetForgotten` _actor _stimulus))))

(fn `HandleSightPerception`
  (params (Actor :type "Actor Object Reference") (Stimulus :type "AIStimulus Structure"))
  (locals (BlackBoard_Target :type Name :default "TargetActor"))
  (bind _actor (`local.Actor`))
  (bind _controlled_bp_zombiepawn (`self.Controlled BP_ZombiePawn`))
  (bind _stimulus (`local.Stimulus`))
  (bind ((`ExpirationAge` _expirationage)) (break `AIStimulus` (`local.Stimulus`)))
  (if (`.bSuccessfullySensed` (break `AIStimulus` Stimulus))
    (`self.OnTargetSensed` _actor _stimulus)
    (`KismetSystemLibrary.K2_ClearAndInvalidateTimerHandle` (`self.TimerHandle_OnSightTimeout`))
    (set `self.SightForgottenActor` null)
    (set `self.SightForgottenStimulus` (struct))
    (`/Engine/EditorBlueprintResources/StandardMacros.IsValid` _controlled_bp_zombiepawn
      (:`Is Valid`
        (bind _outactors (`KismetSystemLibrary.SphereOverlapActors` (`Actor.K2_GetActorLocation` _controlled_bp_zombiepawn) (`/Game/Zombie/Blueprints/BP_Zombie_Pawn.GroupPerceptionRadius` _controlled_bp_zombiepawn) (`|MakeArray` "ObjectTypeQuery3" :!type "EObjectTypeQuery Enum") "/Game/Zombie/Blueprints/BP_Zombie_Pawn.BP_Zombie_Pawn_C"))
        (for _array_element _outactors
          (bind _asbp_zombie_ai_controller_base (cast `/Game/Zombie/Blueprints/Behavior/BP_Zombie_AiController_Base` (`AIBlueprintHelperLibrary.GetAIController` _array_element)))
          (`/Game/Zombie/Blueprints/Behavior/BP_Zombie_AiController_Base.Event_ForceTarget` _asbp_zombie_ai_controller_base (`local.Actor`)))))
    (else
      (`self.OnTargetLost` _actor _stimulus)
      (if (> _expirationage 0.0)
        (set `self.SightForgottenActor` (`local.Actor`))
        (set `self.SightForgottenStimulus` (`local.Stimulus`))
        (bind _returnvalue (`KismetSystemLibrary.K2_SetTimerDelegate` (`|CreateDelegate` :!event `OnSightTimeout`) _expirationage))
        (set `self.TimerHandle_OnSightTimeout` _returnvalue)))))

(fn `OnSightTimeout`
  (`self.OnTargetForgotten` (`self.SightForgottenActor`) (`self.SightForgottenStimulus`)))

(fn `OnTargetPerceptionUpdated_Event`
  (params (Actor :type "Actor Object Reference") (Stimulus :type "AIStimulus Structure"))
  (bind _stimulus (`local.Stimulus`))
  (bind _actor (`local.Actor`))
  (cast `Pawn` Actor)
  (`self.Switch_AiSense` _stimulus
    (:`Sight`
      (`self.HandleSightPerception` _actor _stimulus))
    (:`Hearing`
      (`self.HandleHearingPerception` _actor _stimulus))))