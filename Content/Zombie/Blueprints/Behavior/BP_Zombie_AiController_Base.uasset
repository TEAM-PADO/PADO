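; Base AI controller for zombies that picks and maintains the behavior tree's target actor.
; Senses stay off until the pawn is ready, its damage and death events are bound, and the tree runs.
; Sight, damage and forced targets favor cheaper complete paths or closer actors, while hearing only fills an empty target.
; A timer clears unsensable targets, and losing sight selects the nearest sensable perceived actor.
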(event `self.ReceiveBeginPlay`
  (bind _aiperception (`self.AIPerception`))
  (bind _aiperception_2 (`self.AIPerception`))
  (`|ExecutionSequence`
    (:`then_0`
      ;[1 1 1] disabling the senses to allow for initialization, this is necessary for when we spawn the zombies
      (`AIPerceptionComponent.SetSenseEnabled` _aiperception_2 "/Script/AIModule.AISense_Sight" false)
      (`AIPerceptionComponent.SetSenseEnabled` _aiperception_2 "/Script/AIModule.AISense_Hearing" false))
    (:`then_1`
      (`self.AwaitCharacterInit`)
      (`|ExecutionSequence`
        (:`then_0`
          ;[1 1 1] Caching the Character Value and Binding to the DamageTaken and Death events
          (bind _asbp_zombie_pawn (cast `/Game/Zombie/Blueprints/BP_Zombie_Pawn` (`self.K2_GetPawn`)))
          (bind _output_get (set `self.ZombieCharacter` _asbp_zombie_pawn))
          (add `/Game/Zombie/Blueprints/BP_Zombie_Pawn.OnDamageTaken` _output_get (`|CreateDelegate` :!event `OnPawnTakeDamage_Event`))
          (add `/Game/Zombie/Blueprints/BP_Zombie_Pawn.OnDeath` _output_get (`|CreateDelegate` :!event `OnPawnDeath_Event`)))
        (:`then_1`
          ;[1 1 1] Run the behavior tree and set the initial spawn location
          (`self.RunBehaviorTree` (`self.BTAsset`))
          (`BlackboardComponent.SetValueAsVector` (`AIBlueprintHelperLibrary.GetBlackboard` null) (`self.Key_SpawnLocation`) (`self.K2_GetActorLocation` (`self.ZombieCharacter`)))
          (`BlackboardComponent.SetValueAsBool` (`AIBlueprintHelperLibrary.GetBlackboard` null) (`self.Key_CanRoam`) (`/Game/Zombie/Blueprints/BP_Zombie_Pawn.ShouldRoam` (`self.ZombieCharacter`))))
        (:`then_2`
          ;[1 1 1] Timer used to check if the current target is valid
          (`KismetSystemLibrary.K2_SetTimer` null "ValidateActiveTarget" 0.5 true))
        (:`then_3`
          ;[1 1 1] initialization is complete we can now enable the senses
          (`AIPerceptionComponent.SetSenseEnabled` _aiperception "/Script/AIModule.AISense_Sight" true)
          (`AIPerceptionComponent.SetSenseEnabled` _aiperception "/Script/AIModule.AISense_Hearing" true))))))

(event `self.BPC_PerceptionHandler.OnTargetSensed`
  (params (Actor :type "Actor Object Reference") (Stimulus :type "AIStimulus Structure"))
  ;[1 1 1] Target Sensed, if we don't have a target set it. If the target is already set then check if the new target is easier to get to, if it is then set this new target as the current target
  (bind _returnvalue (message `/Game/Zombie/Blueprints/BPI_Player.BPI_CanBeSensed` Actor))
  (if _returnvalue
    (`/Game/Zombie/Blueprints/Behavior/BPML_Zombie.Switch_AISenseMacro` Stimulus
      (:`Sight`
        (`self.TryUpdateTargetActorByLowestPathCost` Actor))
      (:`Hearing`
        (`self.TryUpdateTargetActorIfNotSet` Actor)))))

(event `Event_ForceTarget`
  (params (Object :type "Object Object Reference"))
  ;[1 1 1] Force Target (For groups noticing together)
  (bind _returnvalue (message `/Game/Zombie/Blueprints/BPI_Player.BPI_CanBeSensed` Object))
  (if _returnvalue
    (bind _asactor (cast `Actor` Object))
    (`self.TryUpdateTargetActorByLowestPathCost` _asactor)))

(event `self.BPC_PerceptionHandler.OnTargetForgotten`
  (params (Actor :type "Actor Object Reference") (Stimulus :type "AIStimulus Structure"))
  (bind _returnvalue (`AIBlueprintHelperLibrary.GetBlackboard` null))
  (bind _key_targetactor (`self.Key_TargetActor`))
  ;[1 1 1] Current Target is lost, now look through all the percieved targets that can be targeted and select the nearest target to chase
  (`/Game/Zombie/Blueprints/Behavior/BPML_Zombie.Switch_AISenseMacro` Stimulus
    (:`Sight`
      (set `self.MostDamageTaken` 0.0)
      (bind (_returnvalue_2 _bisvalid) (`self.Filter` (`AIPerceptionComponent.GetKnownPerceivedActors` (`self.AIPerception`) null)))
      (if _bisvalid
        (`BlackboardComponent.SetValueAsObject` _returnvalue _key_targetactor (`.ReturnValue` (`GameplayStatics.FindNearestActor` (`self.K2_GetActorLocation`) _returnvalue_2)))
        (else
          (`BlackboardComponent.ClearValue` _returnvalue _key_targetactor))))))

(fn `Filter`
  (params (Actors :type "Array of Actor Object Reference"))
  (returns (ReturnValue :type "Array of Actor Object Reference") (bIsValid :type Boolean))
  (locals (L_ReturnArray :type "Array of Actor Object Reference"))
  (bind _l_returnarray (`local.L_ReturnArray`))
  (if (`KismetArrayLibrary.Array_IsNotEmpty` Actors)
    (for _array_element Actors
      (bind _returnvalue (message `/Game/Zombie/Blueprints/BPI_Player.BPI_CanBeSensed` _array_element))
      (if _returnvalue
        (`KismetArrayLibrary.Array_Add` (`local.L_ReturnArray`) _array_element)))
    (return _l_returnarray (`KismetArrayLibrary.Array_IsNotEmpty` _l_returnarray))
    (else
      (return _ false))))

(fn `OnPawnDeath_Event`
  (`BlackboardComponent.SetValueAsBool` (`AIBlueprintHelperLibrary.GetBlackboard` null) (`self.Key_bIsDead`) true))

(fn `OnPawnTakeDamage_Event`
  (params (Damage :type "Float (double-precision)") (CurrentHealth :type "Float (double-precision)") (InstigatedBy :type "Controller Object Reference") (DamageCauser :type "Actor Object Reference"))
  (bind _returnvalue (`self.K2_GetPawn` InstigatedBy))
  (`/Engine/EditorBlueprintResources/StandardMacros.IsValid` _returnvalue
    (:`Is Valid`
      (if (`self.IsActorBeingDestroyed` _returnvalue)
        _
        (elif (>= (`local.Damage`) (`self.MostDamageTaken`))
          (`self.TryUpdateTargetActorByLowestPathCost` _returnvalue))))))

(fn `TryUpdateTargetActorByLowestPathCost`
  (params (Actor :type "Actor Object Reference"))
  (locals (L_CurrentActor :type "Actor Object Reference"))
  (bind _returnvalue (`self.K2_GetPawn`))
  (bind _returnvalue_2 (`AIBlueprintHelperLibrary.GetBlackboard` null))
  (`/Engine/EditorBlueprintResources/StandardMacros.IsValid` _returnvalue_2
    (:`Is Valid`
      (bind _asactor (cast `Actor` (`BlackboardComponent.GetValueAsObject` _returnvalue_2 (`self.Key_TargetActor`)))
        (:`then`
          (set `local.L_CurrentActor` _asactor)
          (`/Engine/EditorBlueprintResources/StandardMacros.IsValid` (`AIBlueprintHelperLibrary.GetCurrentPath` self) ; Are we actively chasing the target?
            (:`Is Valid`
              ;[1 1 1] If the path to the new Actor is easier than the current Path than select the New Actor as the Target Actor
              (bind _returnvalue_3 (`NavigationSystemV1.FindPathToLocationSynchronously` (`self.K2_GetActorLocation` (`self.K2_GetPawn`)) (`self.K2_GetActorLocation` (`local.Actor`)) self "/Script/AIModule.NavFilter_AIControllerDefault"))
              (if (and (< (`NavigationPath.GetPathCost` _returnvalue_3) (`NavigationPath.GetPathCost` (`AIBlueprintHelperLibrary.GetCurrentPath` self))) (not (`NavigationPath.IsPartial` _returnvalue_3)))
                (`BlackboardComponent.SetValueAsObject` (`AIBlueprintHelperLibrary.GetBlackboard` null) (`self.Key_TargetActor`) (`local.Actor`))))
            (:`Is Not Valid`
              ;[1 1 1] If the new Actor is closer than the current Target Actor then set the new Actor as the Targe Actor
              (if (> (`self.GetDistanceTo` (`local.L_CurrentActor`) _returnvalue) (`self.GetDistanceTo` _returnvalue (`local.Actor`)))
                (`BlackboardComponent.SetValueAsObject` (`AIBlueprintHelperLibrary.GetBlackboard` null) (`self.Key_TargetActor`) (`local.Actor`))))))
        (:`CastFailed`
          ;[1 1 1] We don't have a Target Actor so we set the incoming actor as the target
          (`BlackboardComponent.SetValueAsObject` (`AIBlueprintHelperLibrary.GetBlackboard` null) (`self.Key_TargetActor`) (`local.Actor`)))))))

(fn `TryUpdateTargetActorIfNotSet`
  (params (Actor :type "Actor Object Reference"))
  ;[1 1 1] If we don't have an active target, we set the new Actor as the current Target
  (`/Engine/EditorBlueprintResources/StandardMacros.IsValid` (`BlackboardComponent.GetValueAsObject` (`AIBlueprintHelperLibrary.GetBlackboard` null) (`self.Key_TargetActor`))
    (:`Is Not Valid`
      (`BlackboardComponent.SetValueAsObject` (`AIBlueprintHelperLibrary.GetBlackboard` null) (`self.Key_TargetActor`) (`local.Actor`)))))

(fn `UserConstructionScript`)

(fn `ValidateActiveTarget`
  (bind _returnvalue (`BlackboardComponent.GetValueAsObject` (`AIBlueprintHelperLibrary.GetBlackboard` null) (`self.Key_TargetActor`)))
  (`/Engine/EditorBlueprintResources/StandardMacros.IsValid` _returnvalue
    (:`Is Valid`
      (bind _returnvalue_2 (message `/Game/Zombie/Blueprints/BPI_Player.BPI_CanBeSensed` _returnvalue))
      (if (not _returnvalue_2)
        (`BlackboardComponent.ClearValue` (`AIBlueprintHelperLibrary.GetBlackboard` null) (`self.Key_TargetActor`))))))