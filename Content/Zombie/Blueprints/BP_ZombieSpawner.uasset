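; BP_ZombieSpawner spawns a group of BP_Zombie_Pawn zombies around itself when its Spawn event is called.
; A loop based on NumberOfZombies seeks random reachable navmesh points within SpawnRadius, retrying after a short Delay when none is found.
; Each zombie gets a random yaw and the spawner's settings for speed type, material, sounds, health and attack damage.
; Random-scale nodes are unconnected, so zombies spawn at unit scale.
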(event `Spawn`
  (bind (_randomlocation _returnvalue) (`NavigationSystemV1.K2_GetRandomReachablePointInRadius` (`self.K2_GetActorLocation`) (`self.SpawnRadius`) null null))
  (for _ (range (+ (- (`self.NumberOfZombies`) -1) 1))
    (if _returnvalue :!label _label
      (`|SpawnActorFromClass` :`Class` "/Game/Zombie/Blueprints/BP_Zombie_Pawn.BP_Zombie_Pawn_C" :`SpawnTransform` (`KismetMathLibrary.MakeTransform` _randomlocation (`KismetMathLibrary.MakeRotator` 0.0 0.0 (`KismetMathLibrary.RandomFloatInRange` 0.0 360.0))) :`CollisionHandlingOverride` "AdjustIfPossibleButAlwaysSpawn" :`TransformScaleMethod` "MultiplyWithRoot" :`SlowZombie` (`self.Slow Zombie`) :`Material` (`self.Material`) :`AmbientSound` (`self.Ambience Sound`) :`ChasingSound` (`self.Chasing Sound`) :`DeathSound` (`self.Death Sound`) :`Health` (`self.Health`) :`AttackDamage` (`self.Attack Damage`) :`SlashSound` "/Game/Zombie/Sound/SC_Slash.SC_Slash" :`Instigator` null)
      (else
        (`KismetSystemLibrary.Delay` 0.1)
        (goto _label)))))

(fn `UserConstructionScript`)