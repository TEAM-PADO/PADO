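; Zombie appearance randomizer that varies body type and mouth pose on the parent actor's skeletal mesh tagged ZombieMesh.
; Construction and BeginPlay both apply a random or selected regular, muscular or skinny type through morph targets, material and optional actor scale.
; Jaw morphs are then set to a manual pose, a random static pose, or a timeline animation with tongue, started at a random time to desynchronize instances.
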(event `Event_JawPose`
  (bind _returnvalue (`SkeletalMeshComponent.GetAnimInstance` (`self.SkeletalMesh`)))
  (bind _returnvalue_2 (`SkeletalMeshComponent.GetAnimInstance` (`self.SkeletalMesh`)))
  ;[1 0 0] Jaw Open
  (switch `/Game/Zombie/Blueprints/CharacterCreatorSimple/Enum_ZombieMouth` (`self.MouthType`)
    (:`NewEnumerator1`
      (`TimelineComponent.SetNewTime` (`self.Timeline_MouthAnim`) (`KismetMathLibrary.RandomFloatInRange` 0.0 11.0))
      (bind (_direction _jawopen _tongeout) (`Timeline|Timeline_MouthAnim`)
        (:`Update`
          (`AnimInstance.SetMorphTarget` _returnvalue "JawOpen" _jawopen)
          (`AnimInstance.SetMorphTarget` _returnvalue "TongueOut" _tongeout))))
    (:`NewEnumerator0`
      (`AnimInstance.SetMorphTarget` _returnvalue_2 "JawOpen" (`self.ManualJawPose`))
      (`AnimInstance.SetMorphTarget` _returnvalue_2 "TongueOut" (`self.ManualTonguePose`)))
    (:`NewEnumerator2`
      (`AnimInstance.SetMorphTarget` _returnvalue_2 "JawOpen" (`KismetMathLibrary.FClamp` (`KismetMathLibrary.MultiplyMultiply_FloatFloat` (`KismetMathLibrary.RandomFloatInRange` 0.0 1.0) 1.5))))))

(event `self.ReceiveBeginPlay`
  (`self.CharacterStuff`))

(event `Event_SetupBodyType`
  (bind _returnvalue (`self.BodyTypeSetting` 1.0 0.0 1.0))
  (bind _skeletalmesh (`self.SkeletalMesh`))
  (bind _returnvalue_2 (`SkeletalMeshComponent.GetAnimInstance` _skeletalmesh))
  (bind _returnvalue_3 (`SkeletalMeshComponent.GetAnimInstance` (`self.SkeletalMesh`)))
  (bind _returnvalue_4 (`SkeletalMeshComponent.GetAnimInstance` (`self.SkeletalMesh`)))
  (bind _returnvalue_5 (`SkeletalMeshComponent.GetAnimInstance` (`self.SkeletalMesh`)))
  (`/Engine/EditorBlueprintResources/StandardMacros.IsValid` _returnvalue_2
    (:`Is Valid`
      (`SkeletalMeshComponent.ClearMorphTargets` _skeletalmesh)
      (`AnimInstance.SetMorphTarget` _returnvalue_2 "Morph_Torso_Lopsided" (`self.BodyTypeSetting` 0.0 0.0 1.0))
      (`AnimInstance.SetMorphTarget` _returnvalue_2 "TongeOut" (`self.BodyTypeSetting` 1.0 0.5 1.0))
      (switch `int` (`KismetMathLibrary.SelectInt` (`KismetMathLibrary.RandomIntegerInRange` 0 3) (`self.SelectedBodyType`) (`self.Random_BodyType`))
        (:`1`
          ;[0.09063 0.09063 0.09063] Regular
          (`AnimInstance.SetMorphTarget` _returnvalue_5 "Morph_Character_Type1" (`self.BodyTypeSetting` 1.0 0.5 1.0))
          (`AnimInstance.SetMorphTarget` _returnvalue_5 "Morph_Face_Teeth_Fangs" (`self.BodyTypeSetting` 0.7 0.0 0.7))
          (`self.SetScale` (`KismetMathLibrary.RandomFloatInRange` (`self.RegularScale_Min`) (`self.RegularScale_Max`)))
          (`PrimitiveComponent.SetMaterial` (`self.SkeletalMesh`) 0 (`self.Regular Material`)))
        (:`2`
          ;[1 0 0] Muscular
          (`AnimInstance.SetMorphTarget` _returnvalue_4 "Morph_Character_Type1_Muscle" _returnvalue)
          (`AnimInstance.SetMorphTarget` _returnvalue_4 "Morph_Face_Teeth_Fangs" 0.0)
          (`AnimInstance.SetMorphTarget` _returnvalue_4 "Morph_Face_Teeth_Roots" (`self.BodyTypeSetting` 1.0 0.0 1.0))
          (`self.SetScale` (+ (* _returnvalue 0.1) (`self.MuscularScale`)))
          (`PrimitiveComponent.SetMaterial` (`self.SkeletalMesh`) 0 (`self.Muscular Material`)))
        (:`3`
          ;[0.2867 0 1] Skinny
          (`AnimInstance.SetMorphTarget` _returnvalue_3 "Morph_Character_Type1_Skinny" (`self.BodyTypeSetting` 1.5 0.0 1.5))
          (`AnimInstance.SetMorphTarget` _returnvalue_3 "Morph_Face_Teeth_Fangs" 0.8)
          (`AnimInstance.SetMorphTarget` _returnvalue_3 "Morph_Face_Teeth_Roots" 1.0)
          (`AnimInstance.SetMorphTarget` _returnvalue_3 "Morph_Face_Brain_L" (`self.BodyTypeSetting` 0.7 0.0 1.0))
          (`AnimInstance.SetMorphTarget` _returnvalue_3 "Morph_Face_JawWidth_S" (`self.BodyTypeSetting` 0.7 0.5 1.0))
          (`self.SetScale` (`KismetMathLibrary.RandomFloatInRange` (`self.SkinnyScale_Min`) (`self.SkinnyScale_Max`)))
          (`PrimitiveComponent.SetMaterial` (`self.SkeletalMesh`) 0 (`self.Skinny Material`)))))))

(fn `CharacterStuff`
  (bind _output_get (set `self.SkeletalMesh` (`|GetArrayItem` (`self.GetComponentsByTag` (`self.GetParentActor`) "/Script/Engine.SkeletalMeshComponent" "ZombieMesh"))))
  (`/Engine/EditorBlueprintResources/StandardMacros.IsValid` _output_get
    (:`Is Valid`
      (`self.Event_SetupBodyType`)
      (`self.Event_JawPose`))))

(fn `UserConstructionScript`
  (`self.CharacterStuff`))